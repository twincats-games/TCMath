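; Test actor that compares exponential-decay rotator interpolation across meshes updated at same, half and third FPS.
; A looping timeline curve accelerates a yaw speed that spins AnimatedTarget each update.
; SameFPS, HalfFPS and ThirdFPS events pass their delta time to a shared Interp function, which eases each mesh toward the target's relative rotation using RExponentialDecayInterp.
; The file does not show what triggers those three events.
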(event `self.ReceiveBeginPlay`
  (bind _animatedtarget (`self.AnimatedTarget`))
  (bind (_relativerotation_roll _relativerotation_pitch _relativerotation_yaw) (`KismetMathLibrary.BreakRotator` (`SceneComponent.RelativeRotation` _animatedtarget)))
  (`parent.ReceiveBeginPlay`)
  (bind (_direction _zrotationacceleration) (`Timeline|Timeline` :!label _label)
    (:`Update`
      (bind _output_get (set `self.RotationSpeed` (+ (`self.RotationSpeed`) (* _zrotationacceleration (`GameplayStatics.GetWorldDeltaSeconds`) (`self.RotationAcceleration`)))))
      (`SceneComponent.K2_SetRelativeRotation` _animatedtarget (`KismetMathLibrary.MakeRotator` _relativerotation_roll _relativerotation_pitch (+ _relativerotation_yaw (* _output_get (`GameplayStatics.GetWorldDeltaSeconds`)))) false false))
    (:`Finished`
      (goto _label :!via `PlayFromStart`))))

(event `self.ReceiveTick`
  (params (DeltaSeconds :type "Float (single-precision)"))
  (`parent.ReceiveTick` DeltaSeconds))

(event `self.SameFPS`
  (params (InDeltaTime :type "Float (double-precision)"))
  (`self.Interp` InDeltaTime (`self.SameFPSMesh`)))

(event `self.HalfFPS`
  (params (InDeltaTime :type "Float (double-precision)"))
  (`self.Interp` InDeltaTime (`self.HalfFPSMesh`)))

(event `self.ThirdFPS`
  (params (InDeltaTime :type "Float (double-precision)"))
  (`self.Interp` InDeltaTime (`self.ThirdFPSMesh`)))

(fn `Interp`
  (params (InDeltaTime :type "Float (single-precision)") (InTarget :type "SceneComponent Object Reference"))
  (`SceneComponent.K2_SetRelativeRotation` (`local.InTarget`) (`ExponentialDecayInterpBpUtils.RExponentialDecayInterp` (`SceneComponent.RelativeRotation` InTarget) (`SceneComponent.RelativeRotation` (`self.AnimatedTarget`)) InDeltaTime (`self.InterpolationSpeed`)) false false))

(fn `UserConstructionScript`
  (`parent.UserConstructionScript`))