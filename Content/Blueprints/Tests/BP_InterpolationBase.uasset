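; Base test actor for interpolation that simulates updates at full, half and one-third of the frame rate.
; On BeginPlay it teleports the player pawn to a marker location and faces it toward a camera target.
; Tick calls empty SameFPS, HalfFPS and ThirdFPS events, using frame counters and accumulated delta time for the slower two.
; It also stores a settable interpolation speed.
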(event `SetInterpolationSpeed`
  (params (InInterpolationSpeed :type "Float (double-precision)"))
  (set `self.InterpolationSpeed` InInterpolationSpeed))

(event `self.ReceiveBeginPlay`
  ;[1 1 1] Setting Up the Player Pawn
  (bind _output_get (set `self.PlayerPawn` (`GameplayStatics.GetPlayerPawn` 0)))
  (`self.K2_SetActorLocation` _output_get (`self.GetSceneComponentLocation` (`self.PawnLocation`)) false true)
  (`self.K2_SetActorRotation` (`self.PlayerPawn`) (`KismetMathLibrary.FindLookAtRotation` (`self.K2_GetActorLocation` (`self.PlayerPawn`)) (`self.GetSceneComponentLocation` (`self.CameraTarget`))) false))

(event `self.ReceiveTick`
  (params (DeltaSeconds :type "Float (single-precision)"))
  ;[1 1 1] Ticking the interpolations
  (`self.SameFPS` DeltaSeconds)
  (`|ExecutionSequence`
    (:`then_0`
      (set `self.HalfFPSDeltaTime` (+ (`self.HalfFPSDeltaTime`) DeltaSeconds))
      (bind _result (`/Engine/EditorBlueprintResources/StandardMacros.IncrementInt` (`self.HalfFPSCounter`))
        (:`  `
          (if (== _result 2)
            (set `self.HalfFPSCounter` 0)
            (`self.HalfFPS` (`self.HalfFPSDeltaTime`))
            (set `self.HalfFPSDeltaTime` 0.0)))))
    (:`then_1`
      (set `self.ThirdFPSDeltaTime` (+ (`self.ThirdFPSDeltaTime`) DeltaSeconds))
      (bind _result_2 (`/Engine/EditorBlueprintResources/StandardMacros.IncrementInt` (`self.ThirdFPSCounter`))
        (:`  `
          (if (== _result_2 3)
            (set `self.ThirdFPSCounter` 0)
            (`self.ThirdFPS` (`self.ThirdFPSDeltaTime`))
            (set `self.ThirdFPSDeltaTime` 0.0)))))))

(event `SameFPS`
  (params (InDeltaTime :type "Float (double-precision)")))

(event `HalfFPS`
  (params (InDeltaTime :type "Float (double-precision)")))

(event `ThirdFPS`
  (params (InDeltaTime :type "Float (double-precision)")))

(fn `GetSceneComponentLocation`
  (params (InSceneComponent :type "SceneComponent Object Reference"))
  (returns (AbsoluteLocation :type "Vector Structure"))
  (return (+ (`SceneComponent.RelativeLocation` InSceneComponent) (`self.K2_GetActorLocation`))))

(fn `UserConstructionScript`)