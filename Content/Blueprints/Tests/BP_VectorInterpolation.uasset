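; Test actor that compares exponential-decay vector interpolation at full, half and third frame rates, as its event names indicate.
; A Timeline drives AnimatedTarget's relative location, with a FlipFlop on finish alternating reverse and replay.
; SameFPS, HalfFPS and ThirdFPS events each take a delta time and call Interp on their own mesh.
; Interp eases that mesh toward the target at a fixed Y offset using VExponentialDecayInterp.
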(event `self.ReceiveBeginPlay`
  (`parent.ReceiveBeginPlay`)
  (bind (_direction _locationvector) (`Timeline|Timeline` :!label _label)
    (:`Update`
      (`SceneComponent.K2_SetRelativeLocation` (`self.AnimatedTarget`) _locationvector false false))
    (:`Finished`
      (`/Engine/EditorBlueprintResources/StandardMacros.FlipFlop`
        (:`A`
          (goto _label :!via `Reverse`))
        (:`B`
          (goto _label :!via `PlayFromStart`))))))

(event `self.ReceiveTick`
  (params (DeltaSeconds :type "Float (single-precision)"))
  (`parent.ReceiveTick` DeltaSeconds))

(event `self.SameFPS`
  (params (InDeltaTime :type "Float (double-precision)"))
  (`self.Interp` InDeltaTime (`self.SameFPSMesh`) 200.0))

(event `self.HalfFPS`
  (params (InDeltaTime :type "Float (double-precision)"))
  (`self.Interp` InDeltaTime (`self.HalfFPSMesh`) 400.0))

(event `self.ThirdFPS`
  (params (InDeltaTime :type "Float (double-precision)"))
  (`self.Interp` InDeltaTime (`self.ThirdFPSMesh`) 600.0))

(fn `Interp`
  (params (InDeltaTime :type "Float (single-precision)") (InTarget :type "SceneComponent Object Reference") (YOffset :type "Float (double-precision)"))
  (bind (_relativelocation_x _relativelocation_y _relativelocation_z) (`KismetMathLibrary.BreakVector` (`SceneComponent.RelativeLocation` (`self.AnimatedTarget`))))
  (`SceneComponent.K2_SetRelativeLocation` (`local.InTarget`) (`ExponentialDecayInterpBpUtils.VExponentialDecayInterp` (`SceneComponent.RelativeLocation` InTarget) (`KismetMathLibrary.MakeVector` _relativelocation_x (+ YOffset _relativelocation_y) _relativelocation_z) InDeltaTime (`self.InterpolationSpeed`)) false false))

(fn `UserConstructionScript`
  (`parent.UserConstructionScript`))